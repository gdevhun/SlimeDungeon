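; BP_Stage2ResetManager handles resetting Stage 2.
; On BeginPlay it sets IsStage2 on the game instance and creates a fade widget.
; ResetAllObject restores each BP_Movablebox tagged BoxToReset, moves the player to the Stage2ResetPos-tagged actor and plays the fade-out.
; The player move and fade are nested inside the box loop, so they repeat per box and need at least one tagged box.
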(event `self.ReceiveBeginPlay`
  (bind _asbp_game_instance (cast `/Game/Blueprints/System/BP_GameInstance` (`GameplayStatics.GetGameInstance`)))
  (set `/Game/Blueprints/System/BP_GameInstance.bIsStage2` true _asbp_game_instance)
  (bind _returnvalue (`|CreateWidget` "/Game/UI/WBP_FadeAnimWidget.WBP_FadeAnimWidget_C"))
  (set `self.FadeWidget` _returnvalue))

(event `Reset All Object`
  (bind _fadewidget (`self.FadeWidget`))
  (bind _outactors (`GameplayStatics.GetAllActorsOfClassWithTag` "/Game/Blueprints/BP_Movablebox.BP_Movablebox_C" "BoxToReset"))
  (for _array_element _outactors
    (`/Game/Blueprints/BP_Movablebox.ResetBoxTrans` _array_element)
    (bind _asbp_player (cast `/Game/Blueprints/Player/BP_Player` (`GameplayStatics.GetPlayerCharacter` 0)))
    (bind _outactors_2 (`GameplayStatics.GetAllActorsWithTag` "Stage2ResetPos"))
    (for _array_element_2 _outactors_2
      (`self.K2_SetActorLocation` _asbp_player (`self.K2_GetActorLocation` _array_element_2) false false)
      (`UserWidget.AddToViewport` _fadewidget 0)
      (`/Game/UI/WBP_FadeAnimWidget.PlayFadeOut` _fadewidget))))

(fn `UserConstructionScript`)