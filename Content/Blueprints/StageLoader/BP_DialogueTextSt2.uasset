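; Stage 2 dialogue trigger that plays an NPC conversation when the player overlaps its box, then loads Stage 3.
; Overlap freezes movement and flags talking in the game instance; UpdateDialogue steps through parallel text, name and portrait arrays in a widget.
; ExitDialogue restores walking, sets a graphic-manager code flag, then async-loads and opens the next level after a delay.
; Separate events provide a fade-out widget and a timeline-animated outline radius around the player.
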(event `self.ReceiveBeginPlay`
  (bind _returnvalue (`|CreateWidget` "/Game/UI/WBP_DialogueWidget.WBP_DialogueWidget_C"))
  (bind _output_get (set `self.DialogueUI` _returnvalue))
  (`TextBlock.SetText` (`/Game/UI/WBP_DialogueWidget.NPCName` _output_get) (`|GetArrayItem` (`self.NPCNames`) (`self.DialIndex`)))
  (bind _asbp_game_instance (cast `/Game/Blueprints/System/BP_GameInstance` (`GameplayStatics.GetGameInstance`)))
  (set `self.BP Game Instance` _asbp_game_instance))

(event `UpdateDialogue`
  (bind _dialogueui (`self.DialogueUI`))
  (bind _returnvalue (`KismetArrayLibrary.Array_Length` (`self.DialogueList`)))
  (`/Engine/EditorBlueprintResources/StandardMacros.DecrementInt` _returnvalue
    (:`  `
      (if (== (`self.DialIndex`) _returnvalue)
        (`self.ExitDialogue`)
        (else
          (`UserWidget.AddToViewport` _dialogueui 0)
          (`TextBlock.SetText` (`/Game/UI/WBP_DialogueWidget.Text` _dialogueui) (`|GetArrayItem` (`self.DialogueList`) (`self.DialIndex`)))
          (`TextBlock.SetText` (`/Game/UI/WBP_DialogueWidget.NPCName` _dialogueui) (`|GetArrayItem` (`self.NPCNames`) (`self.DialIndex`)))
          (`Image.SetBrushFromTexture` (`/Game/UI/WBP_DialogueWidget.CharImage` (`self.DialogueUI`)) (`|GetArrayItem` (`self.Image`) (`self.DialIndex`)) false)
          (`/Engine/EditorBlueprintResources/StandardMacros.IncrementInt` (`self.DialIndex`)))))))

(event `ExitDialogue`
  (bind _bp_game_instance (`self.BP Game Instance`))
  (`Widget.RemoveFromParent` (`self.DialogueUI`))
  (set `self.DialIndex` 0)
  (`CharacterMovementComponent.SetMovementMode` (`Character.CharacterMovement` (`GameplayStatics.GetPlayerCharacter` 0)) "MOVE_Walking" 0)
  (set `/Game/Blueprints/System/BP_GameInstance.bIsTalking` false _bp_game_instance)
  (set `/Game/Blueprints/System/BP_GameInstance.IsGetGraphicManagerCode` true _bp_game_instance)
  (`GameplayStatics.PlaySound2D` "/Game/Audio/SFX/break_sound_two.break_sound_two" 1.0 1.0 0.0 null null)
  (`KismetSystemLibrary.Delay` 1.0)
  (bind _object (`|LoadAsset` "/Game/Maps/Stage3.Stage3")
    (:`Completed`
      (`GameplayStatics.OpenLevel` (`KismetStringLibrary.Conv_StringToName` (`KismetSystemLibrary.GetDisplayName` _object))))))

(event `Fade`
  (bind _returnvalue (`|CreateWidget` "/Game/UI/WBP_FadeStage1EndAnimWidget.WBP_FadeStage1EndAnimWidget_C"))
  (`UserWidget.AddToViewport` _returnvalue 0)
  (`/Game/UI/WBP_FadeStage1EndAnimWidget.PlayFadeOut` _returnvalue))

(event `self.Box.OnComponentBeginOverlap`
  (params (OverlappedComponent :type "PrimitiveComponent Object Reference") (OtherActor :type "Actor Object Reference") (OtherComp :type "PrimitiveComponent Object Reference") (OtherBodyIndex :type Integer) (bFromSweep :type Boolean) (SweepResult :type "HitResult Structure (by ref)"))
  (cast `/Game/Blueprints/Player/BP_Player` OtherActor)
  (if (not (`self.bIsOnTrigger`))
    (set `self.bIsOnTrigger` false)
    (`GameplayStatics.PlaySound2D` "/Game/Audio/SFX/Item_get_sound.Item_get_sound" 1.0 1.0 0.0 null null)
    (`self.UpdateDialogue`)
    (`CharacterMovementComponent.DisableMovement` (`Character.CharacterMovement` (`GameplayStatics.GetPlayerCharacter` 0)))
    (set `/Game/Blueprints/System/BP_GameInstance.bIsTalking` true (`self.BP Game Instance`))))

(event `self.Box.OnComponentEndOverlap`
  (params (OverlappedComponent :type "PrimitiveComponent Object Reference") (OtherActor :type "Actor Object Reference") (OtherComp :type "PrimitiveComponent Object Reference") (OtherBodyIndex :type Integer))
  (cast `/Game/Blueprints/Player/BP_Player` OtherActor)
  (set `self.bIsOnTrigger` true))

(event `TickBackOuline`
  (`KismetMaterialLibrary.SetVectorParameterValue` "/Game/Designer/Materials/Outline/PC_Outline.PC_Outline" "Position" (`KismetMathLibrary.Conv_VectorToLinearColor` (`SceneComponent.K2_GetComponentLocation` (`Character.CapsuleComponent` (`GameplayStatics.GetPlayerCharacter` 0)))))
  (`/Engine/EditorBlueprintResources/StandardMacros.FlipFlop`
    (:`A`
      (bind (_direction _newtrack_0) (`Timeline|Timeline` :!label _label)
        (:`Update`
          (`KismetMaterialLibrary.SetScalarParameterValue` "/Game/Designer/Materials/Outline/PC_Outline.PC_Outline" "Radius" _newtrack_0))))
    (:`B`
      (goto _label :!via `Reverse`))))

(fn `UserConstructionScript`)