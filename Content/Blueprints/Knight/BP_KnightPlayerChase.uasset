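; BP_KnightPlayerChase is a trigger that ends Stage 1 when the player overlaps its Box.
; The overlap adds the stage-end and fade widgets, plays a fade-out, and disables the player's movement and capsule collision.
; After a short delay, it async-loads the GameMenu asset and opens that level using the loaded asset's display name.
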(event `self.Box.OnComponentBeginOverlap`
  (params (OverlappedComponent :type "PrimitiveComponent Object Reference") (OtherActor :type "Actor Object Reference") (OtherComp :type "PrimitiveComponent Object Reference") (OtherBodyIndex :type Integer) (bFromSweep :type Boolean) (SweepResult :type "HitResult Structure (by ref)"))
  (cast `/Game/Blueprints/Player/BP_Player` OtherActor)
  (bind _returnvalue (`|CreateWidget` "/Game/UI/WBP_Stage1End.WBP_Stage1End_C"))
  (`UserWidget.AddToViewport` _returnvalue 0)
  (bind _returnvalue_2 (`|CreateWidget` "/Game/UI/WBP_FadeEndAnimWidget.WBP_FadeEndAnimWidget_C"))
  (`UserWidget.AddToViewport` _returnvalue_2 0)
  (`/Game/UI/WBP_FadeEndAnimWidget.PlayFadeOut` _returnvalue_2)
  (bind _asbp_player (cast `/Game/Blueprints/Player/BP_Player` (`GameplayStatics.GetPlayerPawn` 0)))
  (`CharacterMovementComponent.DisableMovement` (`Character.CharacterMovement` _asbp_player))
  (`PrimitiveComponent.SetCollisionEnabled` (`Character.CapsuleComponent` _asbp_player) "NoCollision")
  (`KismetSystemLibrary.Delay` 4.0)
  (bind _object (`|LoadAsset` "/Game/Maps/GameMenu.GameMenu")
    (:`Completed`
      (`GameplayStatics.OpenLevel` (`KismetStringLibrary.Conv_StringToName` (`KismetSystemLibrary.GetDisplayName` _object))))))

(fn `UserConstructionScript`)