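; A pushable box that slides along the X or Y axis when BP_Player overlaps it.
; The player's dominant forward axis sets the direction; a sphere trace for WorldDynamic obstacles and a dot-product angle check reject blocked or off-angle pushes.
; A valid push plays a sound and runs a Timeline that moves the box incrementally, with IsMoving guarding against retriggers.
; ResetBoxTrans returns the box to its BeginPlay location and clears movement state.
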(event `self.ReceiveBeginPlay`
  (set `self.IsMoving` false)
  (set `self.FirstTransform` (`self.K2_GetActorLocation`)))

(event `ResetBoxTrans`
  (set `self.IsMoving` false)
  (`self.K2_SetActorLocation` (`self.FirstTransform`))
  (set `self.NotMovePos` false)
  (set `self.MoveDirection` (0.0 0.0)))

(event `self.Box.OnComponentBeginOverlap`
  (params (OverlappedComponent :type "PrimitiveComponent Object Reference") (OtherActor :type "Actor Object Reference") (OtherComp :type "PrimitiveComponent Object Reference") (OtherBodyIndex :type Integer) (bFromSweep :type Boolean) (SweepResult :type "HitResult Structure (by ref)"))
  (bind _returnvalue (`SceneComponent.K2_GetComponentLocation` (`self.Box`)))
  (bind _asbp_player (cast `/Game/Blueprints/Player/BP_Player` OtherActor))
  ;[1 1 1] Abs로 두 벡터 중 더 큰수를 비교, Sign을 통해 부호를 기억해서 가져옴 => MoveDirection Set
  (if (not (`self.IsMoving`))
    (bind (_returnvalue_x _returnvalue_y) (`KismetMathLibrary.BreakVector` (`SceneComponent.GetForwardVector` (`Actor.RootComponent` _asbp_player))))
    (if (> (`KismetMathLibrary.Abs` _returnvalue_x) (`KismetMathLibrary.Abs` _returnvalue_y))
      (set `self.MoveDirection` (`KismetMathLibrary.MakeVector2D` (`KismetMathLibrary.SignOfFloat` _returnvalue_x)))
      (else
        (set `self.MoveDirection` (`KismetMathLibrary.MakeVector2D` 0.0 (`KismetMathLibrary.SignOfFloat` _returnvalue_y)))))
    (bind (_outhit _returnvalue_2) (`KismetSystemLibrary.SphereTraceSingleForObjects` :`Start` _returnvalue :`End` (+ _returnvalue (* (`self.MoveDirection`) (110.0 110.0))) :`Radius` 50.0 :`ObjectTypes` (`|MakeArray` "ObjectTypeQuery2" :!type "EObjectTypeQuery Enum") :`DrawDebugType` "ForDuration"))
    ;[1 1 1] NotMovePos(45도차이가나는지)->(false)  Hit(되었는지 false여야 이동 가능) ->false  NOR => true, true
    (bind _output_get (set `self.NotMovePos` (>= (`KismetMathLibrary.Acos` (`KismetMathLibrary.DotProduct2D` (`self.MoveDirection`) (`KismetMathLibrary.Conv_VectorToVector2D` (`KismetMathLibrary.Vector_Normal2D` (- (`self.K2_GetActorLocation`) (`self.K2_GetActorLocation` (`GameplayStatics.GetPlayerPawn` 0))))))) 0.707)))
    (if (`KismetMathLibrary.BooleanNOR` _output_get _returnvalue_2)
      (if (not (`self.IsMoving`))
        (`GameplayStatics.PlaySound2D` "/Game/Audio/SFX/Boxmove_sound.Boxmove_sound" 1.0 1.0 0.0 null null)
        ;[1 1 1] Timeline을 통해서 벽을 2.5초에 걸쳐서 자연스럽게 이동시킴
        (bind (_direction _float) (`Timeline|Timeline` :!via `PlayFromStart`)
          (:`Update`
            (`self.K2_SetActorLocation` (`KismetMathLibrary.VLerp` (`self.K2_GetActorLocation`) (+ (`self.K2_GetActorLocation`) (* (`self.MoveDirection`) (6.5 6.5))) _float)))
          (:`Finished`
            (set `self.IsMoving` false))
          (:`Event`
            (set `self.IsMoving` true)))))))

(fn `UserConstructionScript`)