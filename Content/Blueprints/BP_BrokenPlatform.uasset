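; BP_BrokenPlatform is a platform that collapses shortly after the player steps on it, then reappears.
; Overlapping its Box with BP_Player plays a warning sound, swaps the material and, after a short delay, shakes the camera.
; When the timer ends, it spawns BP_DestructiblePlatform in its place, plus hides and disables the original.
; After another delay it restores visibility and collision, resets the material and plays the collapse sound.
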(event `self.ReceiveBeginPlay`
  (set `self.FirstTrans` (`self.GetTransform`)))

(event `SetDestructibleUnActive`)

(event `SetDestructibleActive`
  (`|SpawnActorFromClass` "/Game/Blueprints/BP_DestructiblePlatform.BP_DestructiblePlatform_C" (`self.GetTransform`) "Undefined" "MultiplyWithRoot" null null)
  (`ActorComponent.SetActive` (`self.OriginalPlatform`) false false)
  (`ActorComponent.SetActive` (`self.Box`) false false)
  (`SceneComponent.SetVisibility` (`self.OriginalPlatform`) false false)
  (`PrimitiveComponent.SetCollisionEnabled` (`self.Box`) "NoCollision")
  (`PrimitiveComponent.SetCollisionEnabled` (`self.OriginalPlatform`) "NoCollision")
  (`KismetSystemLibrary.Delay` 3.0)
  (`ActorComponent.SetActive` (`self.OriginalPlatform`) true false)
  (`ActorComponent.SetActive` (`self.Box`) true false)
  (`PrimitiveComponent.SetCollisionEnabled` (`self.Box`) "QueryAndPhysics")
  (`PrimitiveComponent.SetCollisionEnabled` (`self.OriginalPlatform`) "QueryAndPhysics")
  (`SceneComponent.SetVisibility` (`self.OriginalPlatform`) true false)
  (`PrimitiveComponent.SetMaterial` (`self.OriginalPlatform`) 0 "/Game/Designer/Modeling/map/stage3/BrokenStone_A01_Mat.BrokenStone_A01_Mat"))

(event `StartTimer`
  (`|ExecutionSequence`
    (:`then_0`
      (`GameplayStatics.PlaySound2D` "/Game/Audio/SFX/BrokenPlatform.BrokenPlatform" 1.0 1.0 0.0 null null))
    (:`then_1`
      (`KismetSystemLibrary.Delay` 3.0)
      (`self.SetDestructibleActive`)
      (`GameplayStatics.PlaySound2D` "/Game/Audio/SFX/Collapse01.Collapse01" 1.0 1.0 0.0 null null))))

(event `self.Box.OnComponentBeginOverlap`
  (params (OverlappedComponent :type "PrimitiveComponent Object Reference") (OtherActor :type "Actor Object Reference") (OtherComp :type "PrimitiveComponent Object Reference") (OtherBodyIndex :type Integer) (bFromSweep :type Boolean) (SweepResult :type "HitResult Structure (by ref)"))
  (cast `/Game/Blueprints/Player/BP_Player` OtherActor)
  (`self.StartTimer`)
  (`PrimitiveComponent.SetMaterial` (`self.OriginalPlatform`) 0 "/Game/Designer/Materials/M_barrier.M_barrier")
  (`KismetSystemLibrary.Delay` 1.0)
  (`PlayerCameraManager.StartCameraShake` :`self` (`GameplayStatics.GetPlayerCameraManager` 0) :`ShakeClass` "/Game/Blueprints/Player/BP_CameraShake.BP_CameraShake_C"))

(fn `UserConstructionScript`)